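; Breakable explosive barrel that takes damage and blows up when its health runs out.
; BeginPlay randomizes the mesh's mass and vertical center-of-mass offset, so each barrel behaves differently under physics.
; Each hit plays a 2D bang and lowers Health; at zero, a short random delay precedes detonation.
; Detonation, also callable directly through the explode event, spawns an Explosion actor, plays an attenuated sound and destroys the barrel.
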(event Custom|explode
  (bind _sm_explosivebarrel (Variables|Default|GetSM_ExplosiveBarrel))
  (Game|SpawnActorfromClass "/Game/Blueprints/ExplodingBarrel/Explosion.Explosion_C" (Transformation|GetWorldTransform _sm_explosivebarrel) "Undefined" "OverrideRootScale" self 3e+02 0)
  (Audio|PlaySoundatLocation "/Game/PrototypeWeap/Sound/RocketLauncher/RL_Explosion_Cue.RL_Explosion_Cue" (Transformation|GetWorldLocation _sm_explosivebarrel) "0, 0, 0" 1.0 1.0 0.0 "/Game/PrototypeWeap/Sound/Attenuation/Explosion_att.Explosion_att" 0 0 0)
  (Actor|DestroyActor))

(event EventBeginPlay
  (bind _sm_explosivebarrel (Variables|Default|GetSM_ExplosiveBarrel))
  (Class|PrimitiveComponent|SetCenterOfMass _sm_explosivebarrel (Math|Vector|MakeVector 0.0 0.0 (Math|Random|RandomFloatinRange 0.0 -5e+01)) "None")
  (Class|PrimitiveComponent|SetMassOverrideinKg _sm_explosivebarrel "None" (Math|Random|RandomFloatinRange 3e+02 6e+02) true))

(event Collision|EventActorBeginOverlap
  (params (OtherActor :type Actor%20Object%20Reference)))

(event EventTick
  (params (DeltaSeconds :type Float%20%28single-precision%29)))

(event EventTakeDamage
  (params (Damage :type Integer) (hitlocation :type Vector :default "0, 0, 0") (impulseLocation :type Vector :default "0, 0, 0") (knockback%20amount :type Integer))
  (bind _sm_explosivebarrel (Variables|Default|GetSM_ExplosiveBarrel))
  (Audio|PlaySound2D "/Game/Audio/steel_drum_bangs.steel_drum_bangs" 1.0 1.0 0.0 0 0)
  (bind _output_get (Variables|Default|Sethealth (- (Variables|Default|Gethealth) Damage)))
  (if (<= _output_get 0)
    (Utilities|FlowControl|Delay (Math|Random|RandomFloatinRange 0.1 0.5))
    (Game|SpawnActorfromClass "/Game/Blueprints/ExplodingBarrel/Explosion.Explosion_C" (Transformation|GetWorldTransform _sm_explosivebarrel) "Undefined" "OverrideRootScale" self 3e+02 0)
    (Audio|PlaySoundatLocation "/Game/PrototypeWeap/Sound/RocketLauncher/RL_Explosion_Cue.RL_Explosion_Cue" (Transformation|GetWorldLocation _sm_explosivebarrel) "0, 0, 0" 1.0 1.0 0.0 "/Game/PrototypeWeap/Sound/Attenuation/Explosion_att.Explosion_att" 0 0 0)
    (Actor|DestroyActor)))

(fn ConstructionScript)