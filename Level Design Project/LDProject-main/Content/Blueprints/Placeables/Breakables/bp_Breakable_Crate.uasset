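; Breakable crate placeable that loses health when damaged and can drop an ammo or health pickup when destroyed.
; Each hit plays a 2D wood sound; at zero health it spawns optional loot and a wood particle effect, then destroys itself.
; Flags choose random ammo, health, or the configured ammo type, with random ammo taking priority and weighted toward one type by a repeated select option.
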(event EventBeginPlay)

(event Collision|EventActorBeginOverlap
  (params (OtherActor :type Actor%20Object%20Reference)))

(event EventTick
  (params (DeltaSeconds :type Float%20%28single-precision%29)))

(event EventTakeDamage
  (params (Damage :type Integer) (hitlocation :type Vector :default "0, 0, 0") (impulseLocation :type Vector :default "0, 0, 0") (knockback%20amount :type Integer))
  (bind _mesh (Variables|Default|GetMesh))
  (bind _returnvalue (Transformation|GetWorldLocation _mesh))
  (bind _output_get (Variables|Default|Sethealth (- (Variables|Default|Gethealth) Damage)))
  (Audio|PlaySound2D "/Game/Audio/wood_hit1_Cue.wood_hit1_Cue" 1.0 1.0 0.0 0 0)
  (if (<= _output_get 0)
    (if (Variables|Default|Getdrop%20loot)
      (if (Variables|Default|GetRandom%20Ammo)
        (Game|SpawnActorfromClass "/Game/Blueprints/Placeables/bp_AmmoPickUp.bp_AmmoPickUp_C" (Math|Transform|MakeTransform _returnvalue "0, 0, 0" "1.000000,1.000000,1.000000") "Undefined" "MultiplyWithRoot" 0 (Utilities|Select :Index (Math|Random|RandomIntegerinRange 0 3) :Option%200 "NewEnumerator1" :Option%201 "NewEnumerator0" :Option%202 "NewEnumerator2" :Option%203 "NewEnumerator0") true 0)
        (elif (Variables|Default|GethealthDrop)
          (Game|SpawnActorfromClass "/Game/Blueprints/Placeables/bp_HealthPcikUp.bp_HealthPcikUp_C" (Math|Transform|MakeTransform _returnvalue "0, 0, 0" "1.000000,1.000000,1.000000") "Undefined" "MultiplyWithRoot" 0 0)
          (else
            (Game|SpawnActorfromClass "/Game/Blueprints/Placeables/bp_AmmoPickUp.bp_AmmoPickUp_C" (Math|Transform|MakeTransform _returnvalue "0, 0, 0" "1.000000,1.000000,1.000000") "Undefined" "MultiplyWithRoot" 0 (Variables|Default|GetAmmotype) true 0)))))
    (Effects|SpawnEmitteratLocation "/Game/GrenadePack/Particles/Wood.Wood" _returnvalue)
    (Actor|DestroyActor)))

(fn ConstructionScript)