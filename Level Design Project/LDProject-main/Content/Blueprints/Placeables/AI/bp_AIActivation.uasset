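; Placeable trigger volume that activates a list of AI when the player enters and handles their reinforcements and cinematics.
; Overlap spawns each AI's controller once and registers this actor as its SpawnManager.
; The Reinforcements event removes AI from the list and, at a count threshold, spawns pistol, rifle and shotgun AI at random locations with shuffled patrol points.
; A sequence plays alongside reinforcements or at its own threshold, disabling player input for cutscenes.
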(event OnComponentBeginOverlap(Box)
  (params (OverlappedComponent :type Primitive%20Component%20Object%20Reference) (OtherActor :type Actor%20Object%20Reference) (OtherComp :type Primitive%20Component%20Object%20Reference) (OtherBodyIndex :type Integer) (bFromSweep :type Boolean) (SweepResult :type Hit%20Result%20Structure%20%28by%20ref%29))
  ;[1 1 1] activate AI
  (if (== OtherActor (Game|GetPlayerCharacter 0))
    (Utilities|FlowControl|DoOnce false
      (:Completed
        (for _array_element (Variables|ActivateAI|GetAI%20to%20Activate)
          (Utilities|IsValid _array_element
            (:Is%20Valid
              (Pawn|SpawnDefaultController _array_element)
              (Variables|/Game/Blueprints/Placeables/AI/bp_AI_ALS_Pistol.bp_AI_ALS_Pistol_C|SetSpawnManager _array_element self))))))))

(event Custom|Reinforcements
  (params (AI%20to%20remove :type Bp%20AI%20ALS%20Pistol%20Object%20Reference))
  (bind _reinforecment_patrolpoint (Variables|Reinforcements|GetReinforecment%20PatrolPoint))
  (bind _reinforecment_patrolpoint_2 (Variables|Reinforcements|GetReinforecment%20PatrolPoint))
  (bind _reinforecment_patrolpoint_3 (Variables|Reinforcements|GetReinforecment%20PatrolPoint))
  ;[1 1 1] call reinforcements
  (Utilities|Array|RemoveItem (Variables|ActivateAI|GetAI%20to%20Activate) AI%20to%20remove)
  (if (<= (Utilities|Array|Length (Variables|ActivateAI|GetAI%20to%20Activate)) (Variables|Reinforcements|Get%20ReinforcementCallNumber))
    (Utilities|FlowControl|DoOnce false
      (:Completed
        (if (Variables|Cinematic|GetCinematicStandalone)
          _
          (elif (Variables|Cinematic|GetIsCutscene)
            ;[1 1 1] Play Cinematic along with reinforcements
            (Utilities|FlowControl|Delay (Variables|Cinematic|GetCinematicStartDelay))
            (CallFunction|PlayCutscene)
            (else
              (Utilities|FlowControl|Delay (Variables|Cinematic|GetCinematicStartDelay))
              (CallFunction|StartCinematic))))
        ;[1 1 1] Sapwn Pistol
        (Utilities|FlowControl|Delay (Variables|Reinforcements|GetReinforcementDelay))
        (for _index (range 0 (- (Variables|Reinforcements|GetReinforcementPistolSpawnAmount) 1))
          (bind _spawn_transform (Utilities|SpawnAI)
            (:Is%20Valid
              (Utilities|Array|Shuffle _reinforecment_patrolpoint)
              (bind _returnvalue (Game|SpawnActorfromClass "/Game/Blueprints/Placeables/AI/bp_AI_ALS_Pistol.bp_AI_ALS_Pistol_C" _spawn_transform "AdjustIfPossibleButAlwaysSpawn" "SelectDefaultAtRuntime" 0 _reinforecment_patrolpoint (Variables|Reinforcements|GetSpawn%20and%20See%20Player) true 0))
              (Pawn|SpawnDefaultController (Variables|/Script/Engine.Actor|GetInstigator _returnvalue)))))
        ;[1 1 1] Spawn Rifle
        (for _index_2 (range 0 (- (Variables|Reinforcements|GetReinforcementRifleSpawnAmount) 1))
          (bind _spawn_transform_2 (Utilities|SpawnAI)
            (:Is%20Valid
              (Utilities|Array|Shuffle _reinforecment_patrolpoint_2)
              (bind _returnvalue_2 (Game|SpawnActorfromClass "/Game/Blueprints/Placeables/AI/bp_AI_ALS_Rifle.bp_AI_ALS_Rifle_C" _spawn_transform_2 "AdjustIfPossibleButAlwaysSpawn" "SelectDefaultAtRuntime" 0 _reinforecment_patrolpoint_2 (Variables|Reinforcements|GetSpawn%20and%20See%20Player) true 0))
              (Pawn|SpawnDefaultController (Variables|/Script/Engine.Actor|GetInstigator _returnvalue_2)))))
        ;[1 1 1] Spawn Shotgun
        (for _index_3 (range 0 (- (Variables|Reinforcements|GetReinforcementShotgunSpawnAmount) 1))
          (bind _spawn_transform_3 (Utilities|SpawnAI)
            (:Is%20Valid
              (Utilities|Array|Shuffle _reinforecment_patrolpoint_3)
              (bind _returnvalue_3 (Game|SpawnActorfromClass "/Game/Blueprints/Placeables/AI/bp_ALS_ShotgunAI.bp_ALS_ShotgunAI_C" _spawn_transform_3 "AdjustIfPossibleButAlwaysSpawn" "SelectDefaultAtRuntime" 0 _reinforecment_patrolpoint_3 (Variables|Reinforcements|GetSpawn%20and%20See%20Player) true 0))
              (Pawn|SpawnDefaultController (Variables|/Script/Engine.Actor|GetInstigator _returnvalue_3)))))))
    (else
      ;[1 1 1] Check to see if cinematic should play independant of reinforcement number
      (if (and (<= (Utilities|Array|Length (Variables|ActivateAI|GetAI%20to%20Activate)) (Variables|Cinematic|GetCinematicCallNumber)) (Variables|Cinematic|GetCinematicStandalone))
        (Utilities|FlowControl|DoOnce false
          (:Completed
            (Utilities|FlowControl|Delay (Variables|Cinematic|GetCinematicStartDelay))
            (if (Variables|Cinematic|GetIsCutscene)
              (CallFunction|PlayCutscene)
              (else
                (CallFunction|StartCinematic)))))))))

(event Custom|PlayCutscene
  (bind _sequence_to_play (Variables|Cinematic|GetSequence%20to%20play))
  (bind _sequenceplayer (Variables|/Script/LevelSequence.LevelSequenceActor|GetSequencePlayer _sequence_to_play))
  (Utilities|IsValid _sequence_to_play
    (:Is%20Valid
      (Sequencer|Player|Play _sequenceplayer :!class /Script/MovieScene.MovieSceneSequencePlayer)
      (Input|DisableInput (Game|GetPlayerCharacter 0) (Game|GetPlayerController 0))
      (Utilities|FlowControl|Delay (Class|TimeManagementBlueprintLibrary|ToSeconds(QualifiedFrameTime) (Class|MovieSceneSequencePlayer|GetEndTime _sequenceplayer)))
      (Input|EnableInput (Game|GetPlayerCharacter 0) (Game|GetPlayerController 0)))))

(event EventBeginPlay)

(event Collision|EventActorBeginOverlap
  (params (OtherActor :type Actor%20Object%20Reference)))

(event EventTick
  (params (DeltaSeconds :type Float%20%28single-precision%29)))

(fn ConstructionScript
  (bind _textrender (Variables|Default|GetTextRender))
  (Transformation|SetRelativeScale3D _textrender (/ (Variables|/Script/Engine.SceneComponent|GetRelativeScale3D _textrender) (Transformation|GetActorScale3D)))
  (Transformation|SetWorldLocation (Variables|Default|GetTextRender) (.Origin (Collision|GetComponentBounds (Variables|Default|GetBox))) false false))

(fn StartCinematic
  (bind _sequence_to_play (Variables|Cinematic|GetSequence%20to%20play))
  (Utilities|IsValid _sequence_to_play
    (:Is%20Valid
      (Sequencer|Player|Play (Variables|/Script/LevelSequence.LevelSequenceActor|GetSequencePlayer _sequence_to_play) :!class /Script/MovieScene.MovieSceneSequencePlayer))))