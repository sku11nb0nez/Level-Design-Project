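; Interactable elevator that rides a spline between two ends, toggled by interaction or sent up or down remotely.
; A trigger closes the linked top/bottom doors and the sliding internal door, then a looping timer moves the car at constant interp speed.
; On arrival it plays sounds, opens the doors and repositions the interaction highlight and box.
; The construction script builds hidden-in-game spline meshes along the path and sets the car's start position.
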(event Custom|MoveElevator
  (Variables|Default|SetCurrentPosition (Math|Interpolation|FInterptoConstant (Variables|Default|GetCurrentPosition) (select (Variables|Default|GetMovingUp) (Spline|GetSplineLength (Variables|Default|GetSpline)) 0.0) (Utilities|Time|GetWorldDeltaSeconds) (Variables|Default|GetInterp%20Speed)))
  (if (Math|Float|NearlyEqual(Float) (Math|Interpolation|FInterptoConstant (Variables|Default|GetCurrentPosition) (select (Variables|Default|GetMovingUp) (Spline|GetSplineLength (Variables|Default|GetSpline)) 0.0) (Utilities|Time|GetWorldDeltaSeconds) (Variables|Default|GetInterp%20Speed)) (select (Variables|Default|GetMovingUp) (Spline|GetSplineLength (Variables|Default|GetSpline)) 0.0) 0.01)
    (Utilities|Time|ClearandInvalidateTimerbyHandle (Variables|Default|GetElevatorTimer))
    (CallFunction|DoorSetuponCompleted)
    (Audio|Components|Audio|FadeOut (Variables|Default|GetElevatortraveling) 1.5 0.0 "Linear" :!class /Script/Engine.AudioComponent)
    (Audio|PlaySoundatLocation "/Game/BlockingStarterPack/Blueprints/AutomaticDoor/ElevatorCompleted.ElevatorCompleted" (Transformation|GetWorldLocation (Variables|Default|Get%20Mesh)) "0, 0, 0" 1.0 1.0 0.0 0 0 0 0)
    (CallFunction|OpenInternalDoor true)
    (Audio|PlaySoundatLocation "/Game/BlockingStarterPack/Blueprints/AutomaticDoor/elevatorDing.elevatorDing" (Transformation|GetWorldLocation (Variables|Default|Get%20Mesh)) "0, 0, 0" 1.0 1.0 0.0 0 0 0 0)
    (else
      (Transformation|SetRelativeLocation (Variables|Default|Get%20Mesh) (Spline|GetLocationatDistanceAlongSpline (Variables|Default|GetSpline) (Variables|Default|GetCurrentPosition) "Local") false false))))

(event Custom|OpenInternalDoor
  (params (open :type Boolean))
  (bind _elevatordoor (Variables|Default|GetElevatorDoor))
  (bind _elevatordoor_2 (Variables|Default|GetElevatorDoor))
  (bind _elevatordoor_3 (Variables|Default|GetElevatorDoor))
  (bind _relativelocation (Variables|/Script/Engine.SceneComponent|GetRelativeLocation _elevatordoor_2))
  (bind _relativescale3d (Variables|/Script/Engine.SceneComponent|GetRelativeScale3D _elevatordoor))
  (if open
    (bind _movement (Timeline|Timeline_0 PlayFromStart)
      (:Update
        (Transformation|SetRelativeLocation _elevatordoor_3 (Math|Vector|Lerp(Vector) (Math|Vector|MakeVector -12.742257 (.y _relativelocation) (.z _relativelocation)) (Math|Vector|MakeVector 3e+01 (.y _relativelocation) (.z _relativelocation)) _movement) false false)
        (Transformation|SetRelativeScale3D _elevatordoor_3 (Math|Vector|Lerp(Vector) (Math|Vector|MakeVector 0.707543 (.y _relativescale3d) (.z _relativescale3d)) (Math|Vector|MakeVector 0.2 (.y _relativescale3d) (.z _relativescale3d)) _movement))))
    (else
      (Timeline|Timeline_0 ReverseFromEnd))))

(event EventBeginPlay
  (|CallParentFunction)
  (Audio|Components|Audio|FadeOut (Variables|Default|GetElevatortraveling) 0.01 0.0 "Linear" :!class /Script/Engine.AudioComponent))

(event Collision|EventActorBeginOverlap
  (params (OtherActor :type Actor%20Object%20Reference))
  (|CallParentFunction OtherActor) ; This node is disabled and will not be called.\nDrag off pins to build functionality.
)

(event EventTick
  (params (DeltaSeconds :type Float%20%28single-precision%29))
  (|CallParentFunction DeltaSeconds) ; This node is disabled and will not be called.\nDrag off pins to build functionality.
)

(event EventRemoteInteractResponse
  (if (Variables|Default|GetMovingUp)
    (Variables|Default|SetMovingUp false)
    (else
      (Variables|Default|SetMovingUp true)))
  (Utilities|FlowControl|Sequence
    (:then_0
      (Utilities|FlowControl|DoOnce false :!label _label
        (:Completed
          (Audio|PlaySoundatLocation "/Game/BlockingStarterPack/Blueprints/AutomaticDoor/ElevatorCompleted.ElevatorCompleted" (Transformation|GetWorldLocation (Variables|Default|Get%20Mesh)) "0, 0, 0" 1.0 1.0 0.0 0 0 0 0)
          (Audio|Components|Audio|FadeIn (Variables|Default|GetElevatortraveling) 0.5 1.0 0.0 "Linear" :!class /Script/Engine.AudioComponent)
          (bind _topdoors (Variables|Default|GetTopDoors)
            (:then
              (Default|CloseDoor _topdoors)
              (bind _bottomdoors (Variables|Default|GetBottomDoors)
                (:then
                  (Default|CloseDoor _bottomdoors)
                  (Development|SetHiddeninGame (Variables|Default|Get%20Highlight) true false)
                  (CallFunction|OpenInternalDoor false))
                (:else)))
            (:else)))))
    (:then_1
      (Utilities|FlowControl|Delay 0.5)
      (bind _returnvalue (Utilities|Time|SetTimerbyEvent (delegate Custom|MoveElevator) 0.01 true))
      (Variables|Default|SetElevatorTimer _returnvalue)
      (goto _label Reset))))

(event EventRemoteInteract
  (params (Direction :type EDirection%20Enum :default "Left"))
  (switch Utilities|FlowControl|Switch|SwitchonEDirection Direction
    (:Up
      (Variables|Default|SetMovingUp true))
    (:Down
      (Variables|Default|SetMovingUp false)))
  (Utilities|FlowControl|Sequence
    (:then_0
      (Utilities|FlowControl|DoOnce false :!label _label
        (:Completed
          (Audio|PlaySoundatLocation "/Game/BlockingStarterPack/Blueprints/AutomaticDoor/ElevatorCompleted.ElevatorCompleted" (Transformation|GetWorldLocation (Variables|Default|Get%20Mesh)) "0, 0, 0" 1.0 1.0 0.0 0 0 0 0)
          (Audio|Components|Audio|FadeIn (Variables|Default|GetElevatortraveling) 0.5 1.0 0.0 "Linear" :!class /Script/Engine.AudioComponent)
          (bind _topdoors (Variables|Default|GetTopDoors)
            (:then
              (Default|CloseDoor _topdoors)
              (bind _bottomdoors (Variables|Default|GetBottomDoors)
                (:then
                  (Default|CloseDoor _bottomdoors)
                  (Development|SetHiddeninGame (Variables|Default|Get%20Highlight) true false)
                  (CallFunction|OpenInternalDoor false))
                (:else)))
            (:else)))))
    (:then_1
      (Utilities|FlowControl|Delay 0.5)
      (bind _returnvalue (Utilities|Time|SetTimerbyEvent (delegate Custom|MoveElevator) 0.01 true))
      (Variables|Default|SetElevatorTimer _returnvalue)
      (goto _label Reset))))

(fn ConstructionScript
  (bind _spline (Variables|Default|GetSpline))
  (bind _spline_2 (Variables|Default|GetSpline))
  (|CallParentFunction)
  (for _index (range 0 (- (Spline|GetNumberOfSplinePoints (Variables|Default|GetSpline)) 2))
    (bind _returnvalue (AddComponent|AddSplineMeshComponent false))
    (Components|StaticMesh|SetStaticMesh _returnvalue "/Game/BlockOut/Shapes/Static_Meshes/Cylinder.Cylinder")
    (SplineMesh|SetForwardAxis _returnvalue (Variables|Default|GetAxis) true)
    (Transformation|AttachComponentToComponent _returnvalue (Variables|Default|GetSpline) "None" "KeepRelative" "KeepRelative" "KeepRelative" true)
    (SplineMesh|SetStartandEnd _returnvalue (Spline|GetLocationatSplinePoint _spline_2 _index "Local") (Spline|GetTangentatSplinePoint _spline_2 _index "Local") (Spline|GetLocationatSplinePoint _spline_2 (+ _index 1) "Local") (Spline|GetTangentatSplinePoint _spline_2 (+ _index 1) "Local") true :!class /Script/Engine.SplineMeshComponent)
    (Development|SetHiddeninGame _returnvalue true false)
    (Rendering|Components|TextRender|SetText (Variables|Default|GetTextRender) (Utilities|Text|ToText(String) (Utilities|String|Append (Utilities|String|ToString(Float) (Variables|ElevatorSettings|GetPlayRate%20seconds)) " Seconds")))
    (Transformation|SetRelativeLocation (Variables|Default|Get%20Mesh) (Spline|GetLocationatSplinePoint _spline (select (Variables|ElevatorSettings|GetMoveToEnd) (Spline|GetNumberOfSplinePoints _spline) 0) "Local") false false)))

(fn DoorSetuponCompleted
  (bind __highlight (Variables|Default|Get%20Highlight))
  (bind _box (Variables|Default|GetBox))
  (bind __mesh (Variables|Default|Get%20Mesh))
  (bind _relativelocation (Variables|/Script/Engine.SceneComponent|GetRelativeLocation _box))
  (bind _relativelocation_2 (Variables|/Script/Engine.SceneComponent|GetRelativeLocation __mesh))
  (bind _relativelocation_3 (Variables|/Script/Engine.SceneComponent|GetRelativeLocation __highlight))
  (bind _returnvalue (+ (.z _relativelocation_2) 2e+02))
  (if (Variables|Default|GetMovingUp)
    (bind _topdoors (Variables|Default|GetTopDoors)
      (:then
        (Default|OpenDoor _topdoors))
      (:else))
    (else
      (bind _bottomdoors (Variables|Default|GetBottomDoors)
        (:then
          (Default|OpenDoor _bottomdoors))
        (:else))))
  (Transformation|SetRelativeLocation __highlight (Math|Vector|MakeVector (.x _relativelocation_3) (.y _relativelocation_3) _returnvalue) false false)
  (Transformation|SetRelativeLocation (Variables|Default|GetBox) (Math|Vector|MakeVector (.x _relativelocation) (.y _relativelocation) _returnvalue) false false)
  (Development|SetHiddeninGame (Variables|Default|Get%20Highlight) false false))