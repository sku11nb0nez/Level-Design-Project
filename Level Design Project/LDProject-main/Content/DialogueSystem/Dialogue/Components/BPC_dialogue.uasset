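; BPC_dialogue is an actor component that gives its owner full dialogue and brief brush-past speech.
; Speak creates WBP_Dialogue with the speaker, lines, greeting sound and component reference, ends any active brush-past, then opens it through OpenWidget.
; BrushPast shows WBP_BrushPast on the owner's WidgetComponent when lines exist.
; A finished-dialogue dispatcher drives EndBrushPastDialogue, which unbinds and clears that widget.
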(event Custom|Speak
  ;[1 1 1] Creates the dialogue widget
  (bind _returnvalue (UserInterface|CreateWidget "/Game/DialogueSystem/Dialogue/Widgets/WBP_Dialogue.WBP_Dialogue_C" 0 (Variables|Default|GetSpeakersName) (Variables|Default|GetDialogue) (Variables|Default|GetGreetingDialogue) self))
  ;[1 1 1] If brushing past or triggering open world speaking then cancels playing sound. for best effect use 2 different sounds such as a "come here" and then a "hello"
  (Variables|Default|GetBrushPastWidget
    (:then
      (CallFunction|EndBrushPastDialogue))
    (:else
      _))
  ;[1 1 1] Global function to open widget
  (CallFunction|OpenWidget _returnvalue))

(event Custom|BrushPast
  (bind _returnvalue (Components|GetOwner))
  (bind _returnvalue_2 (Actor|GetComponentbyClass _returnvalue "/Script/UMG.WidgetComponent"))
  ;[1 1 1] Creates the brush past widget and feeds required text
  (if (> (Utilities|Array|Length (Variables|Default|GetBrushPastDialogue)) 0)
    (bind _returnvalue_3 (UserInterface|CreateWidget "/Game/DialogueSystem/Dialogue/Widgets/WBP_BrushPast.WBP_BrushPast_C" 0 (Variables|Default|GetSpeakersName) (Variables|Default|GetBrushPastDialogue) (Variables|Default|GetBrushPastGreeting) (Variables|Default|GetText%20Delay)))
    (bind _output_get (Variables|Default|SetBrushPastWidget _returnvalue_3))
    ;[1 1 1] Sets widget to be visible and to the brushg past widget
    (Utilities|IsValid _returnvalue_2
      (:Is%20Valid
        (UserInterface|SetWidget _returnvalue_2 _output_get)
        (Rendering|SetVisibility _returnvalue_2 true false)
        ;[1 1 1] Binds to when the event has finished
        (EventDispatchers|BindEventtoOnFinishedDialogue _returnvalue_3 (EventDispatchers|CreateEvent :!event Custom|EndBrushPastDialogue)))
      (:Is%20Not%20Valid
        (Development|PrintString "Widget Not valid")))
    (else
      (Development|PrintString "No dialogue to display"))))

(event Custom|EndBrushPastDialogue
  (bind _returnvalue (Components|GetOwner))
  (bind _returnvalue_2 (Actor|GetComponentbyClass _returnvalue "/Script/UMG.WidgetComponent"))
  ;[1 1 1] Linked to the disatcher. unbinds to stop listening to future events. Ends the speach and returns the widget to not being set and not visible
  (Variables|Default|GetBrushPastWidget
    (:then
      (EventDispatchers|UnbindEventfromOnFinishedDialogue (Variables|Default|GetBrushPastWidget) (delegate Custom|EndBrushPastDialogue))
      (UserInterface|SetWidget _returnvalue_2 0)
      (Rendering|SetVisibility _returnvalue_2 true false)
      (Variables|Default|SetBrushPastWidget 0))
    (:else)))